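; Character selection Blueprint that swaps the skeletal mesh it displays among a list of character meshes.
; The ChangeCharacter event increments the current index, wrapping to zero after the last entry in the Character array, and sets the Mesh component's skeletal mesh asset from that array.
; The construction script is empty.
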(event Custom|Change%20Character
  (if (< (Variables|Default|GetCurrentcharacterindex) (- (Utilities|Array|Length (Variables|Default|GetCharacter)) 1))
    (bind _result (Math|Integer|IncrementInt (Variables|Default|GetCurrentcharacterindex))
      (:%20%20
        _))
    (else
      (Variables|Default|SetCurrentcharacterindex 0)))
  (Components|SkeletalMesh|SetSkeletalMeshAsset (Variables|Default|GetMesh) (Utilities|Array|Get(acopy) (Variables|Default|GetCharacter) _result)))

(fn ConstructionScript)