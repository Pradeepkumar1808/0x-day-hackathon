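; BP_Enemy is a sword-wielding enemy, optionally a boss, with a health component linked to a widget bar, plus montage-driven sword and big attacks.
; A looping timer drives sphere traces between sword points, switched for bosses, applying damage behind a DoOnce reset after a delay.
; A separate radial point trace deals fixed damage.
; Incoming damage reduces health, while Die disables movement, ragdolls the mesh and blocks sword traces.
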(event Custom|Damage%20Trace
  (if (not (Variables|Default|GetisDead?))
    (bind _outhit (Collision|SphereTraceForObjects (Math|Vector|SelectVector (Variables|Default|GetbossStart%20sword%20trace%20boss) (Transformation|GetWorldLocation (Variables|Default|GetStart%20%20sword%20Trace)) (Variables|Default|Getisboss?)) (Math|Vector|SelectVector (Variables|Default|GetbossEndsword%20trace%20boss_0) (Transformation|GetWorldLocation (Variables|Default|GetEnd%20%20sword%20Trace1)) (Variables|Default|Getisboss?)) 25.0 (Utilities|Array|MakeArray "ObjectTypeQuery3") false 0 "ForOneFrame"))
    (if true
      (Utilities|FlowControl|DoOnce false :!label _label
        (:Completed
          (Game|Damage|ApplyDamage (.HitActor (Collision|BreakHitResult _outhit)) (Variables|Default|GetSword%20Damage) 0 0)
          (Utilities|FlowControl|Delay 0.3)
          (goto _label Reset))))))

(event EventPointDamageTrace
  (bind _outhit (Collision|SphereTraceForObjects (Transformation|GetWorldLocation (Variables|Default|GetPoint%20Trace%20Pos)) "0, 0, 0" (Variables|Default|GetPoint%20Attack%20Radius) (Utilities|Array|MakeArray "ObjectTypeQuery3") false 0 "ForDuration" true "(R=1.000000,G=0.000000,B=0.000000,A=1.000000)" "(R=0.000000,G=1.000000,B=0.000000,A=1.000000)" 1.0))
  (if true
    (Game|Damage|ApplyDamage (.HitActor (Collision|BreakHitResult _outhit)) 1e+01 0 0)))

(event EventBeginSwordTrace
  (bind _returnvalue (Utilities|Time|SetTimerbyEvent (delegate Custom|Damage%20Trace) 0.1 true)))

(event EventEndSwordTrace0
  (if (Utilities|Time|IsValidTimerHandle (stale EventBeginSwordTrace _returnvalue))
    (Utilities|Time|ClearandInvalidateTimerbyHandle (stale EventBeginSwordTrace _returnvalue))))

(event EventBeginPlay
  (bind _aswb_enemyr_health_1 (Utilities|Casting|CastToWb_EnemyrHealth1 (UserInterface|GetWidget (Variables|Default|GetWidget))))
  (Default|SetHealthProgressBar (Variables|Default|GetBpc_Health) (Variables|/Game/UI/Wb_EnemyrHealth1.Wb_EnemyrHealth1_C|GetHealthBar _aswb_enemyr_health_1)))

(event Game|Damage|EventAnyDamage
  (params (Damage :type Float%20%28single-precision%29) (DamageType :type Damage%20Type%20Object%20Reference) (InstigatedBy :type Controller%20Object%20Reference) (DamageCauser :type Actor%20Object%20Reference))
  (Default|IncreaseValues (Variables|Default|GetBpc_Health) "NewEnumerator0" (* Damage -1.0)))

(event EventDie
  (Pawn|Components|CharacterMovement|DisableMovement (Variables|Character|GetCharacterMovement))
  (Physics|SetSimulatePhysics (Variables|Character|GetMesh) true)
  (Variables|Default|SetisDead? true))

(fn ConstructionScript)

(fn BigAttack
  (bind _returnvalue (Animation|PlayAnimMontage (Variables|Default|Getbig%20attack%20montage) 1.0 "None"))
  (return _returnvalue))

(fn SwordAttack
  (bind _returnvalue (Animation|PlayAnimMontage (Variables|Default|GetSword%20attack%20montage) 1.0 "None"))
  (return _returnvalue))